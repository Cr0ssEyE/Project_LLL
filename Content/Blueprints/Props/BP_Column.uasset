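; BP_Column is a breakable column prop that reacts to damage caused by the player's pawn.
; The first hit hides Column01 and hands collision to Column02, and the next hides Column02.
; Each hit also reveals RockBase, plays a spike-move timeline on it, and sphere-traces nearby.
; Monster capsule hits trigger ApplyDamage, though no damaged actor is wired into that call.
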(event EventBeginPlay
  (Transformation|SetRelativeScale3D (Variables|Default|GetRockBase) "0, 0, 0"))

(event Collision|EventActorBeginOverlap
  (params (OtherActor :type Actor%20Object%20Reference)))

(event EventTick
  (params (DeltaSeconds :type Float%20%28single-precision%29)))

(event Game|Damage|EventAnyDamage
  (params (Damage :type Float%20%28single-precision%29) (DamageType :type Damage%20Type%20Object%20Reference) (InstigatedBy :type Controller%20Object%20Reference) (DamageCauser :type Actor%20Object%20Reference))
  (bind _returnvalue (Transformation|GetActorLocation))
  (bind _column01 (Variables|Default|GetColumn01))
  (bind _column02 (Variables|Default|GetColumn02))
  (if (== DamageCauser (Pawn|GetControlledPawn (Game|GetPlayerController 0)))
    (Utilities|FlowControl|Sequence
      (:then_0
        (if (Rendering|IsVisible (Variables|Default|GetColumn01))
          (Rendering|SetVisibility _column01 false false)
          (Collision|SetCollisionProfileName _column02 "Monster" true :!class /Script/Engine.PrimitiveComponent)
          (Collision|SetCollisionProfileName _column01 "NoCollision" true :!class /Script/Engine.PrimitiveComponent)
          (else
            (Rendering|SetVisibility _column02 false false)
            (Collision|SetCollisionProfileName _column02 "NoCollision" true :!class /Script/Engine.PrimitiveComponent))))
      (:then_1
        (bind _spikemoveslider (Timeline|타임라인 Play)
          (:Update
            (Transformation|SetRelativeLocation (Variables|Default|GetRockBase) (Math|Vector|Lerp(Vector) (Variables|Default|GetStartLocation) (Variables|Default|GetEndLocation) _spikemoveslider) false false))))
      (:then_2
        (Transformation|SetRelativeScale3D (Variables|Default|GetRockBase) "1.000000,1.000000,1.000000")
        (bind _outhits (Collision|MultiSphereTraceByChannel _returnvalue _returnvalue 1.5e+02 "TraceTypeQuery4" false 0 "None"))
        (for _array_element _outhits
          (Utilities|Casting|CastToLLL_MonsterBase (.HitActor (Collision|BreakHitResult _array_element)))
          (Utilities|Casting|CastToCapsuleComponent (.HitComponent (Collision|BreakHitResult _array_element)))
          (Game|Damage|ApplyDamage 0 3e+01 0 0))))))

(fn ConstructionScript)