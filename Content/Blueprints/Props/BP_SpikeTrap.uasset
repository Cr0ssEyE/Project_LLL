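; Spike trap prop that damages the player when their controlled pawn enters its trigger box.
; After a short delay, a timeline lerps the spike mesh from start to end location, then resets its time on finish.
; As the spike starts moving, a box trace at the actor's location applies fixed damage to LLL_PlayerBase hits on capsule components only.
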(event OnComponentBeginOverlap(Box)
  (params (OverlappedComponent :type Primitive%20Component%20Object%20Reference) (OtherActor :type Actor%20Object%20Reference) (OtherComp :type Primitive%20Component%20Object%20Reference) (OtherBodyIndex :type Integer) (bFromSweep :type Boolean) (SweepResult :type Hit%20Result%20Structure%20%28by%20ref%29))
  (bind _returnvalue (Transformation|GetActorLocation))
  (if (== OtherActor (Pawn|GetControlledPawn (Game|GetPlayerController 0)))
    (Utilities|FlowControl|Delay 0.2)
    (Utilities|FlowControl|Sequence
      (:then_0
        (bind _spikemoveslider (Timeline|SpikeMoveTime Play)
          (:Update
            (Transformation|SetRelativeLocation (Variables|Default|GetSpike) (Math|Vector|Lerp(Vector) (Variables|Default|GetStartLocation) (Variables|Default|GetEndLocation) _spikemoveslider) false false))
          (:Finished
            (if true
              (Timeline|SpikeMoveTime SetNewTime)))))
      (:then_1
        (bind _outhits (Class|KismetSystemLibrary|BoxTraceMultibyProfile _returnvalue _returnvalue "100.000000,100.000000,20.000000" "0, 0, 0" "OverlapAll" false (Utilities|Array|MakeArray self) "None" true))
        (for _array_element _outhits
          (bind _aslll_player_base (Utilities|Casting|CastToLLL_PlayerBase (.HitActor (Collision|BreakHitResult _array_element))))
          (Utilities|Casting|CastToCapsuleComponent (.HitComponent (Collision|BreakHitResult _array_element)))
          (Game|Damage|ApplyDamage _aslll_player_base 3e+01 0 0))))))

(event EventBeginPlay)

(event Collision|EventActorBeginOverlap
  (params (OtherActor :type Actor%20Object%20Reference)))

(event EventTick
  (params (DeltaSeconds :type Float%20%28single-precision%29)))

(fn ConstructionScript)