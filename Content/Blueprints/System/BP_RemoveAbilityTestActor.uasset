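; Test actor that strips ability-part gameplay effects from a player who overlaps it.
; On overlap with an LLL_PlayerBase, it removes all stacks of active effects tagged AbilityPart.Dash through the player's Ability System Component.
; The AbilityPart.Common removal is nested inside the Dash loop, so it runs only when Dash effects are found.
; Successful removals print a debug message, and Tick continuously rotates the static mesh.
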(event EventBeginPlay)

(event Collision|EventActorBeginOverlap
  (params (OtherActor :type Actor%20Object%20Reference))
  (bind _aslll_player_base (Utilities|Casting|CastToLLL_PlayerBase OtherActor))
  (bind _returnvalue (GameplayEffects|GetActiveEffectswithAllTags (Ability|GetAbilitySystemComponent _aslll_player_base) (GameplayTags|MakeGameplayTagContainerfromTag "(TagName=\"AbilityPart.Dash\")")))
  (for _array_element _returnvalue
    (bind _returnvalue_2 (GameplayEffects|RemoveActiveGameplayEffect (Ability|GetAbilitySystemComponent _aslll_player_base) _array_element -1))
    (Development|PrintText "Remove Effect" _returnvalue_2 _returnvalue_2)
    (bind _returnvalue_3 (GameplayEffects|GetActiveEffectswithAllTags (Ability|GetAbilitySystemComponent _aslll_player_base) (GameplayTags|MakeGameplayTagContainerfromTag "(TagName=\"AbilityPart.Common\")")))
    (for _array_element_2 _returnvalue_3
      (bind _returnvalue_4 (GameplayEffects|RemoveActiveGameplayEffect (Ability|GetAbilitySystemComponent _aslll_player_base) _array_element_2 -1))
      (Development|PrintText "Remove Effect" _returnvalue_4 _returnvalue_4))))

(event EventTick
  (params (DeltaSeconds :type Float%20%28single-precision%29))
  (Transformation|AddRelativeRotation (Variables|Default|GetStaticMesh) "0.000000,1.000000,0.000000" false false))

(fn ConstructionScript)