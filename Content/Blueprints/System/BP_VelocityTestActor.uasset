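; A debug test character that measures how long CharacterMovement velocity takes to decay after a one-off push.
; BeginPlay drops the Mesh to the capsule's bottom, then after a short delay sets a forward velocity along world X.
; Tick accumulates delta time while the velocity is non-zero and prints the running total.
; A flag cleared shortly after the push and some speed checks are left unused.
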(event EventBeginPlay
  (Transformation|SetRelativeLocation (Variables|Character|GetMesh) (Math|Vector|MakeVector 0.0 0.0 (* (Components|Capsule|GetScaledCapsuleHalfHeight (Variables|Collision|GetCapsuleComponent)) -1.0)) false false)
  (Utilities|FlowControl|Delay 1.0)
  (Variables|/Script/Engine.MovementComponent|SetVelocity (Variables|Character|GetCharacterMovement) "1000.000000,0.000000,0.000000")
  (Utilities|FlowControl|Delay 0.1)
  (Variables|Default|SetNewVar_0 false))

(event Collision|EventActorBeginOverlap
  (params (OtherActor :type Actor%20Object%20Reference)))

(event EventTick
  (params (DeltaSeconds :type Float%20%28single-precision%29))
  (if (not (Math|Vector|VectorIsNearlyZero (Variables|/Script/Engine.MovementComponent|GetVelocity (Variables|Character|GetCharacterMovement))))
    (bind _output_get (Variables|Default|SetNewVar (+ DeltaSeconds (Variables|Default|GetNewVar))))
    (Development|PrintText (Utilities|Text|ToText(Float) _output_get "HalfToEven"))))

(fn ConstructionScript)