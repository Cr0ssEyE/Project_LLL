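; BP_Box is a helper actor in the PC death dissolve VFX folder that publishes an oriented box volume to materials.
; Its construction script writes the Cube component's world location, scale and forward, right and up axes into the PC_Box_Data material parameter collection.
; The event graph is empty, so the values refresh only when the construction script runs, not per frame.
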(event EventBeginPlay)

(event Collision|EventActorBeginOverlap
  (params (OtherActor :type Actor%20Object%20Reference)))

(event EventTick
  (params (DeltaSeconds :type Float%20%28single-precision%29)))

(fn ConstructionScript
  (bind _cube (Variables|Default|GetCube))
  (bind _cube_2 (Variables|Default|GetCube))
  (Rendering|Material|SetVectorParameterValue "/Game/VFX/Base/Particle/PC/State/Death/Dissolve/PC_Box_Data.PC_Box_Data" "Location" (Math|Conversions|ToLinearColor(Vector) (Transformation|GetWorldLocation _cube)) :!class /Script/Engine.KismetMaterialLibrary)
  (Rendering|Material|SetVectorParameterValue "/Game/VFX/Base/Particle/PC/State/Death/Dissolve/PC_Box_Data.PC_Box_Data" "Bounds" (Math|Conversions|ToLinearColor(Vector) (Transformation|GetWorldScale _cube)) :!class /Script/Engine.KismetMaterialLibrary)
  (Rendering|Material|SetVectorParameterValue "/Game/VFX/Base/Particle/PC/State/Death/Dissolve/PC_Box_Data.PC_Box_Data" "X" (Math|Conversions|ToLinearColor(Vector) (Math|Vector|GetForwardVector _cube_2)) :!class /Script/Engine.KismetMaterialLibrary)
  (Rendering|Material|SetVectorParameterValue "/Game/VFX/Base/Particle/PC/State/Death/Dissolve/PC_Box_Data.PC_Box_Data" "Y" (Math|Conversions|ToLinearColor(Vector) (Math|Vector|GetRightVector _cube_2)) :!class /Script/Engine.KismetMaterialLibrary)
  (Rendering|Material|SetVectorParameterValue "/Game/VFX/Base/Particle/PC/State/Death/Dissolve/PC_Box_Data.PC_Box_Data" "Z" (Math|Conversions|ToLinearColor(Vector) (Math|Vector|GetUpVector _cube_2)) :!class /Script/Engine.KismetMaterialLibrary))